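; Game mode that keeps a set of AI characters and commands them as a group to move to the player or stop.
; BeginPlay shows the mouse cursor and sets Game and UI input with lock on capture.
; AddMeToBeActivated adds a character to the set and returns CharacterAlreadyExists, computed as not Contains despite its name.
; The move and stop functions loop over the set, calling each valid AI.
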(event `self.ReceiveBeginPlay`
  (bind _returnvalue (`GameplayStatics.GetPlayerController` 0))
  (`WidgetBlueprintLibrary.SetInputMode_GameAndUIEx` _returnvalue null "LockOnCapture")
  (set `PlayerController.bShowMouseCursor` true _returnvalue))

(fn `AddMeToBeActivated`
  (params (`AI Character` :type "/Game/Blueprint/ThirdPersonAICharacter Object Reference"))
  (returns (Successful :type Boolean))
  (locals (`Character Already Exists?` :type Boolean :default false))
  (bind _ais_to_activate (`self.AIs To Activate`))
  (set `local.Character Already Exists?` (not (`BlueprintSetLibrary.Set_Contains` _ais_to_activate `AI Character`)))
  (`BlueprintSetLibrary.Set_Add` _ais_to_activate `AI Character`)
  (return (`local.Character Already Exists?`)))

(fn `AIs Move to Player`
  (bind _result (`BlueprintSetLibrary.Set_ToArray` (`self.AIs To Activate`)))
  (for _array_element _result
    (`/Engine/EditorBlueprintResources/StandardMacros.IsValid` _array_element
      (:`Is Valid`
        (`/Game/Blueprint/ThirdPersonAICharacter.MoveToPlayer` _array_element)))))

(fn `AIs StopMovement`
  (bind _result (`BlueprintSetLibrary.Set_ToArray` (`self.AIs To Activate`)))
  (for _array_element _result
    (`/Engine/EditorBlueprintResources/StandardMacros.IsValid` _array_element
      (:`Is Valid`
        (`/Game/Blueprint/ThirdPersonAICharacter.Stop Movement` _array_element)))))

(fn `UserConstructionScript`)